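; BP_TrainStop is a train stop trigger that halts BP_Train_Blueprint when it overlaps the Cube, which is hidden at BeginPlay along with its TextRender.
; Each train overlap calls StopRequest; unless FinalStop is set, a DoOnce-guarded delay based on StopPeriod restarts the engines, then resets the guard after another delay.
; A looping timer also fires TraceForTrain, which is empty.
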(event `self.ReceiveBeginPlay`
  (`KismetSystemLibrary.K2_SetTimerDelegate` (delegate `Trace for Train`) 0.1 true)
  (`SceneComponent.SetVisibility` (`self.Cube`) false false)
  (`SceneComponent.SetVisibility` (`self.TextRender`) false false))

(event `Trace for Train`)

(event `self.Cube.OnComponentBeginOverlap`
  (params (OverlappedComponent :type "PrimitiveComponent Object Reference") (OtherActor :type "Actor Object Reference") (OtherComp :type "PrimitiveComponent Object Reference") (OtherBodyIndex :type Integer) (bFromSweep :type Boolean) (SweepResult :type "HitResult Structure (by ref)"))
  (bind _asbp_train_blueprint (cast `/Game/WildWestVillage/AS_WildWest/Train/Blueprints/BP_Train_Blueprint` OtherActor))
  (`/Game/WildWestVillage/AS_WildWest/Train/Blueprints/BP_Train_Blueprint.Stop Request` _asbp_train_blueprint)
  (set `self.As BP Train Blueprint` _asbp_train_blueprint)
  (`/Engine/EditorBlueprintResources/StandardMacros.DoOnce` false :!label _label
    (:`Completed`
      (if (not (`self.Final Stop`))
        (`KismetSystemLibrary.Delay` (+ (`self.Stop_Period`) 15.0))
        (`/Game/WildWestVillage/AS_WildWest/Train/Blueprints/BP_Train_Blueprint.Start the Engines` (`self.As BP Train Blueprint`))
        (`KismetSystemLibrary.Delay` 15.0)
        (goto _label :!via `Reset`)))))

(fn `UserConstructionScript`)