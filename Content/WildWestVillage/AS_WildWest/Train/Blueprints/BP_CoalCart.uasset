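; Coal cart actor for a train, placed along a rail track spline at a distance supplied by its caller.
; Each placement wraps negative distances, applies a height offset and dampens the spline's roll.
; Speed updates and emergency stops use separate timelines to blend speed, feeding a scaled value to the cart's Animation Blueprint.
; Construction-script logic for attaching to a Locomotive is disconnected and never runs.
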(event `self.ReceiveBeginPlay`
  (bind _asabp_coal_cart (cast `/Game/WildWestVillage/AS_WildWest/Train/Anim/ABP_CoalCart` (`SkeletalMeshComponent.GetAnimInstance` (`self.Cart`))))
  (set `/Game/WildWestVillage/AS_WildWest/Train/Anim/ABP_CoalCart.Speed` 0.0 _asabp_coal_cart)
  (set `self.ABP` _asabp_coal_cart))

(event `EmergencyStop`
  (params (Speed :type "Float (double-precision)"))
  (set `self.CachedSpeed` (`self.Speed`))
  (bind (_direction _alpha) (`Timeline|Timeline_1` :!via `PlayFromStart`)
    (:`Update`
      (bind _output_get (set `self.Speed` (`KismetMathLibrary.Lerp` (`self.CachedSpeed`) Speed _alpha)))
      (set `/Game/WildWestVillage/AS_WildWest/Train/Anim/ABP_CoalCart.Speed` (* _output_get 0.1) (`self.ABP`)))
    (:`Finished`
      (set `self.CachedSpeed` (`self.Speed`)))))

(event `Update Speed`
  (params (Speed :type "Float (double-precision)"))
  (bind (_direction _alpha) (`Timeline|Timeline_0` :!via `PlayFromStart`)
    (:`Update`
      (bind _output_get (set `self.Speed` (`KismetMathLibrary.Lerp` (`self.CachedSpeed`) Speed _alpha)))
      (set `/Game/WildWestVillage/AS_WildWest/Train/Anim/ABP_CoalCart.Speed` (* _output_get 0.1) (`self.ABP`)))
    (:`Finished`
      (set `self.CachedSpeed` (`self.Speed`)))))

(event `Update Rail Track`
  (params (`Rail Track` :type "/Game/WildWestVillage/AS_WildWest/Train/Blueprints/BP_Rails Object Reference"))
  (set `self.Rail Track` `Rail Track`))

(event `Rotate Locomtive to Match the Rails Rotation`
  (params (Distance :type "Float (double-precision)") (`Actor Rot` :type "Rotator Structure") (maxDistance :type "Float (double-precision)") (ZAxisOffset :type "Float (double-precision)"))
  (set `self.CartDistance` Distance)
  (if (not (>= Distance 0.0))
    (set `self.CartDistance` (+ Distance maxDistance)))
  (bind _rail_track (`self.Rail Track`)
    (:`then`
      (`self.K2_SetActorTransform` (`KismetMathLibrary.MakeTransform` (+ (.location (`SplineComponent.GetTransformAtDistanceAlongSpline` (`/Game/WildWestVillage/AS_WildWest/Train/Blueprints/BP_Rails.Spline` _rail_track) (`self.CartDistance`) "World" false)) (0.0 0.0 48.0) (`KismetMathLibrary.MakeVector` 0.0 0.0 ZAxisOffset)) (`KismetMathLibrary.MakeRotator` (/ (.roll (.rotation (`SplineComponent.GetTransformAtDistanceAlongSpline` (`/Game/WildWestVillage/AS_WildWest/Train/Blueprints/BP_Rails.Spline` _rail_track) (`self.CartDistance`) "World" false))) (`self.Roll Dampener`)) (.pitch (.rotation (`SplineComponent.GetTransformAtDistanceAlongSpline` (`/Game/WildWestVillage/AS_WildWest/Train/Blueprints/BP_Rails.Spline` _rail_track) (`self.CartDistance`) "World" false))) (.yaw (.rotation (`SplineComponent.GetTransformAtDistanceAlongSpline` (`/Game/WildWestVillage/AS_WildWest/Train/Blueprints/BP_Rails.Spline` _rail_track) (`self.CartDistance`) "World" false)))))))
    (:`else`)))

(fn `UserConstructionScript`
  (bind _locomotive (`self.Locomotive`)
    (:`then`)
    (:`else`)))