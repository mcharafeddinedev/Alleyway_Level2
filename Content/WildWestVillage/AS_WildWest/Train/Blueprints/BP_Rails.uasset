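; BP_Rails is a spline-based track actor that lays rail meshes along an editable path for the WildWest village train set.
; The construction script sets the spline's closed-loop state, then adds a spline mesh component per Spacing interval, using the configured StaticMesh.
; Each segment takes its endpoints from the spline and scales direction by Spacing for tangents, so pieces bend along the curve.
; The event graph has no runtime logic.
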(event `self.ReceiveBeginPlay`)

(event `self.ReceiveTick`
  (params (DeltaSeconds :type "Float (single-precision)")))

(fn `UserConstructionScript`
  (bind _spline (`self.Spline`))
  (bind _spacing (`self.Spacing`))
  (`SplineComponent.SetClosedLoop` (`self.Spline`) (`self.ClosedLoop`) true)
  (for _index (range (+ (`.ReturnValue` (`KismetMathLibrary.FMod` (`SplineComponent.GetSplineLength` (`self.Spline`)) _spacing)) 1))
    (bind _returnvalue (`AddComponent|NODE_AddSplineMeshComponent-1`))
    (`StaticMeshComponent.SetStaticMesh` _returnvalue (`self.StaticMesh`))
    (bind _returnvalue_2 (* _index _spacing))
    (bind _returnvalue_3 (+ _returnvalue_2 _spacing))
    (`SplineMeshComponent.SetStartAndEnd` _returnvalue (`SplineComponent.GetLocationAtDistanceAlongSpline` _spline _returnvalue_2 "Local") (* (`SplineComponent.GetDirectionAtDistanceAlongSpline` _spline _returnvalue_2 "Local") _spacing) (`SplineComponent.GetLocationAtDistanceAlongSpline` _spline _returnvalue_3 "Local") (* (`SplineComponent.GetDirectionAtDistanceAlongSpline` _spline _returnvalue_3 "Local") _spacing) true)))