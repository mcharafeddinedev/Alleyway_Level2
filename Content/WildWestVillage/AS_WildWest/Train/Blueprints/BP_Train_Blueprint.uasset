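; Train locomotive actor that finds the BP_Rails track beneath it, snaps to its spline and drives along it with attached carts.
; A fast looping timer advances distance by speed, wraps on closed tracks or halts at open ends, and positions each cart at a length-based offset behind the engine.
; Timelines ease starts and emergency stops, feeding speed to the carts and locomotive animation Blueprint while toggling steam, smoke and braking particles.
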(event `self.ReceiveBeginPlay`
  ;[0 0.4676 1] Identify Rail track, and snap the train locomotive to that spline track
  (`KismetSystemLibrary.K2_SetTimerDelegate` (delegate `Trace For Rail Track`) 0.1)
  (bind _asabp_train_locomotive_3 (cast `/Game/WildWestVillage/AS_WildWest/Train/Anim/ABP_TrainLocomotive3` (`SkeletalMeshComponent.GetAnimInstance` (`self.SkeletalMeshComponent`))))
  (set `self.ABP` _asabp_train_locomotive_3)
  (`KismetSystemLibrary.Delay` 0.2)
  (`KismetSystemLibrary.K2_SetTimerDelegate` (delegate `Tick Alternative`) 0.005 true))

(event `Trace For Rail Track`
  (bind _returnvalue (`SceneComponent.GetSocketLocation` (`self.SkeletalMeshComponent`) "Train"))
  ;[0 0.4676 1] Identify Rail track, and snap the train locomotive to that spline track
  (bind _outhits (`KismetSystemLibrary.LineTraceMulti` _returnvalue (+ _returnvalue (0.0 0.0 -50.0)) "TraceTypeQuery1"))
  (set `self.Rail Track` null)
  (for _array_element _outhits
    (bind _asbp_rails (cast `/Game/WildWestVillage/AS_WildWest/Train/Blueprints/BP_Rails` (`.HitActor` (`GameplayStatics.BreakHitResult` _array_element))))
    (`|ExecutionSequence`
      (:`then_0`
        (break))
      (:`then_1`
        (set `self.Rail Track` _asbp_rails))))
  (bind _rail_track (`self.Rail Track`)
    (:`then`
      (`self.K2_SetActorTransform` (`KismetMathLibrary.MakeTransform` (+ (.location (`SplineComponent.GetTransformAtDistanceAlongSpline` (`/Game/WildWestVillage/AS_WildWest/Train/Blueprints/BP_Rails.Spline` _rail_track) (`self.StartingPosition`) "World" false)) (0.0 0.0 48.0)) (.rotation (`SplineComponent.GetTransformAtDistanceAlongSpline` (`/Game/WildWestVillage/AS_WildWest/Train/Blueprints/BP_Rails.Spline` _rail_track) (`self.StartingPosition`) "World" false))))
      (set `self.DistanceTraveled` (`self.StartingPosition`))
      (if (`/Game/WildWestVillage/AS_WildWest/Train/Blueprints/BP_Rails.ClosedLoop` _rail_track)
        (bind _spline (`/Game/WildWestVillage/AS_WildWest/Train/Blueprints/BP_Rails.Spline` _rail_track))
        (bind _returnvalue_2 (`SplineComponent.GetNumberOfSplinePoints` (`/Game/WildWestVillage/AS_WildWest/Train/Blueprints/BP_Rails.Spline` _rail_track)))
        (set `self.MaxDistance` (`SplineComponent.GetDistanceAlongSplineAtSplinePoint` _spline _returnvalue_2))
        (else
          (set `self.MaxDistance` (`SplineComponent.GetDistanceAlongSplineAtSplinePoint` _spline (- _returnvalue_2 1)))))
      (`self.Start the Engines`)
      (set `self.Looping` (`/Game/WildWestVillage/AS_WildWest/Train/Blueprints/BP_Rails.ClosedLoop` _rail_track))
      ;[0 0.6506 1] Update all Assigned Train Carts to be attached to the train and same specific spline track
      (for (_array_element_2 _array_index) (`self.AttachedCarts`)
        (`/Engine/EditorBlueprintResources/StandardMacros.IsValid` _array_element_2
          (:`Is Valid`
            (switch `int` _array_index
              (:`Default`
                (`self.K2_SetActorLocationAndRotation` :`self` _array_element_2)
                (set `/Game/WildWestVillage/AS_WildWest/Train/Blueprints/BP_CoalCart.AttachCart` (`self.CachedCart`) _array_element_2)
                (bind _output_get (set `self.CachedCart` _array_element_2))
                (`/Game/WildWestVillage/AS_WildWest/Train/Blueprints/BP_CoalCart.Update Rail Track` _output_get (`self.Rail Track`)))
              (:`0`
                (bind _output_get_2 (set `self.CachedCart` _array_element_2))
                (set `/Game/WildWestVillage/AS_WildWest/Train/Blueprints/BP_CoalCart.1st Cart` true _output_get_2)
                (`/Game/WildWestVillage/AS_WildWest/Train/Blueprints/BP_CoalCart.Update Rail Track` _output_get_2 (`self.Rail Track`))))))))
    (:`else`)))

(event `Tick Alternative`
  ;[0 0.4676 1] Identify Rail track, and snap the train locomotive to that spline track
  (`self.Rotate Locomtive to Match the Rails Rotation`)
  (`self.Track Distance Travelled and account for speed`))

(event `Rotate Locomtive to Match the Rails Rotation`
  (bind _returnvalue (`self.K2_GetActorRotation`))
  (bind _distancetraveled (`self.DistanceTraveled`))
  ;[1 1 1] Update Train location on spline based on Distance traveled
  (bind _rail_track (`self.Rail Track`)
    (:`then`
      (`|ExecutionSequence`
        (:`then_0`
          (`self.K2_SetActorTransform` (`KismetMathLibrary.MakeTransform` (+ (.location (`SplineComponent.GetTransformAtDistanceAlongSpline` (`/Game/WildWestVillage/AS_WildWest/Train/Blueprints/BP_Rails.Spline` _rail_track) _distancetraveled "World" false)) (0.0 0.0 48.0) (`KismetMathLibrary.MakeVector` 0.0 0.0 (`self.ZaxisOffset`))) (`KismetMathLibrary.MakeRotator` (/ (.roll (.rotation (`SplineComponent.GetTransformAtDistanceAlongSpline` (`/Game/WildWestVillage/AS_WildWest/Train/Blueprints/BP_Rails.Spline` _rail_track) _distancetraveled "World" false))) (`self.Roll Dampener`)) (.pitch (.rotation (`SplineComponent.GetTransformAtDistanceAlongSpline` (`/Game/WildWestVillage/AS_WildWest/Train/Blueprints/BP_Rails.Spline` _rail_track) _distancetraveled "World" false))) (.yaw (.rotation (`SplineComponent.GetTransformAtDistanceAlongSpline` (`/Game/WildWestVillage/AS_WildWest/Train/Blueprints/BP_Rails.Spline` _rail_track) _distancetraveled "World" false))))))
          ;[1 1 1] Match all Train Carts behind the train at their respective distance based on their length
          (for (_array_element _array_index) (`self.AttachedCarts`)
            (`/Engine/EditorBlueprintResources/StandardMacros.IsValid` _array_element
              (:`Is Valid`
                (switch `int` _array_index
                  (:`Default`
                    (`/Game/WildWestVillage/AS_WildWest/Train/Blueprints/BP_CoalCart.Rotate Locomtive to Match the Rails Rotation` _array_element (- (`self.DistanceTraveled`) (+ (* (+ _array_index 1) (`/Game/WildWestVillage/AS_WildWest/Train/Blueprints/BP_CoalCart.CartLenght` _array_element)) 110.0)) _returnvalue (`self.MaxDistance`) (`self.ZaxisOffset`)))
                  (:`0`
                    (`/Game/WildWestVillage/AS_WildWest/Train/Blueprints/BP_CoalCart.Rotate Locomtive to Match the Rails Rotation` _array_element (- (`self.DistanceTraveled`) (+ (`/Game/WildWestVillage/AS_WildWest/Train/Blueprints/BP_CoalCart.CartLenght` _array_element) 110.0)) _returnvalue (`self.MaxDistance`) (`self.ZaxisOffset`))))))))
        (:`then_1`
          (if (`self.DebugDistance`)
            (`KismetSystemLibrary.PrintString` (`KismetStringLibrary.Conv_DoubleToString` _distancetraveled) true true (struct :`R` 1.0 :`G` 0.265023 :`A` 1.0) 0.1)))))
    (:`else`)))

(event `Track Distance Travelled and account for speed`
  ;[1 1 1] Update Distance Traveled, for the purpose of tracking track loops
  (if (< (`self.DistanceTraveled`) (`self.MaxDistance`))
    (set `self.DistanceTraveled` (+ (`self.DistanceTraveled`) (`self.Speed`)))
    (elif (`self.Looping`)
      (set `self.DistanceTraveled` 0.0)
      (else
        (set `self.Speed` 0.0)
        (set `/Game/WildWestVillage/AS_WildWest/Train/Anim/ABP_TrainLocomotive3.Speed` 0.0 (`self.ABP`))))))

(event `Stop Request`
  ;[1 1 1] Stop request issued, Stop the train
  (set `self.CachedSpeed` (`self.Speed`))
  (`self.EmergencyStop` 0.0))

(event `Update Speed`
  (params (TargetSpeed :type "Float (double-precision)"))
  ;[1 1 1] Keep track of speed and pass that information to relevant animation blueprints
  (`|ExecutionSequence`
    (:`then_0`
      (for _array_element (`self.AttachedCarts`)
        (`/Engine/EditorBlueprintResources/StandardMacros.IsValid` _array_element
          (:`Is Valid`
            (`/Game/WildWestVillage/AS_WildWest/Train/Blueprints/BP_CoalCart.Update Speed` _array_element (* TargetSpeed 6.0))))))
    (:`then_1`
      (bind (_direction _alpha) (`Timeline|Speed Lerp` :!via `PlayFromStart`)
        (:`Update`
          (bind _output_get (set `self.Speed` (`KismetMathLibrary.Lerp` (`self.CachedSpeed`) TargetSpeed _alpha)))
          (set `/Game/WildWestVillage/AS_WildWest/Train/Anim/ABP_TrainLocomotive3.Speed` (* _output_get 0.2) (`self.ABP`)))
        (:`Finished`
          (set `self.CachedSpeed` (`self.Speed`)))))))

(event `EmergencyStop`
  (params (TargetSpeed :type "Float (double-precision)"))
  ;[1 1 1] Stopping logic.  Slow down speed, update all carts and kill relevant VFX
  (`|ExecutionSequence`
    (:`then_0`
      (for _array_element (`self.AttachedCarts`)
        (`/Engine/EditorBlueprintResources/StandardMacros.IsValid` _array_element
          (:`Is Valid`
            (`/Game/WildWestVillage/AS_WildWest/Train/Blueprints/BP_CoalCart.EmergencyStop` _array_element (* TargetSpeed 2.0))))))
    (:`then_1`
      (bind (_direction _alpha) (`Timeline|Timeline_0` :!via `PlayFromStart`)
        (:`Update`
          (bind _output_get (set `self.Speed` (`KismetMathLibrary.Lerp` (`self.CachedSpeed`) TargetSpeed _alpha)))
          (set `/Game/WildWestVillage/AS_WildWest/Train/Anim/ABP_TrainLocomotive3.Speed` (* _output_get 0.1) (`self.ABP`)))
        (:`Finished`
          (set `self.CachedSpeed` (`self.Speed`)))))
    (:`then_2`
      ;;[1 0.704 0] VFX
      (`ActorComponent.Activate` (`self.ParticleSystem2`) true)
      (`ActorComponent.Activate` (`self.ParticleSystem3`) true)
      (`ActorComponent.Activate` (`self.ParticleSystem5`) true)
      (`ActorComponent.Activate` (`self.ParticleSystem4`) true))
    (:`then_3`
      (`KismetSystemLibrary.Delay` 12.0)
      ;;[1 0.6082 0] VFX
      (`ActorComponent.Deactivate` (`self.ParticleSystem3`))
      (`ActorComponent.Deactivate` (`self.ParticleSystem2`))
      (`ActorComponent.Deactivate` (`self.ParticleSystem5`))
      (`ActorComponent.Deactivate` (`self.ParticleSystem4`)))))

(event `Activate Steam`
  ;[1 0.5905 0] VFX events and fluff
  ;;[1 1 1] Activate Steam VFX
  (`|ExecutionSequence`
    (:`then_0`
      (bind (_direction _alpha) (`Timeline|Scale Spawn Particles` :!via `PlayFromStart`)
        (:`Update`
          (`SceneComponent.SetRelativeScale3D` (`self.P_Steam_Lit`) (`KismetMathLibrary.Conv_DoubleToVector` _alpha))
          (`SceneComponent.SetRelativeScale3D` (`self.P_Steam_Lit2`) (`KismetMathLibrary.Conv_DoubleToVector` _alpha))
          (`SceneComponent.SetRelativeScale3D` (`self.ParticleSystem`) (`KismetMathLibrary.Conv_DoubleToVector` _alpha))
          (`SceneComponent.SetRelativeScale3D` (`self.ParticleSystem1`) (`KismetMathLibrary.Conv_DoubleToVector` _alpha)))))
    (:`then_1`
      (`ActorComponent.Activate` (`self.P_Steam_Lit2`) false)
      (`ActorComponent.Activate` (`self.P_Steam_Lit`) false)
      (`ActorComponent.Activate` (`self.ParticleSystem1`) false)
      (`ActorComponent.Activate` (`self.ParticleSystem`) false)
      (`KismetSystemLibrary.Delay` 12.0)
      (`ActorComponent.Deactivate` (`self.P_Steam_Lit2`))
      (`ActorComponent.Deactivate` (`self.P_Steam_Lit`))
      (`ActorComponent.Deactivate` (`self.ParticleSystem1`))
      (`ActorComponent.Deactivate` (`self.ParticleSystem`)))))

(event `Start the Engines`
  ;[1 1 1] Start request issued, activate VFX and start gaining speed
  (`self.Activate Steam `)
  (`self.Update Speed` (`self.AnimationSpeed`))
  ;;[1 0.6913 0] VFX
  (`ActorComponent.Activate` (`self.P_Smoke1`) true)
  (`ActorComponent.Activate` (`self.P_Smoke`) true))

(fn `UserConstructionScript`
  (set `SkeletalMeshComponent.GlobalAnimRateScale` (`self.AnimationSpeed`) (`self.SkeletalMeshComponent`)))