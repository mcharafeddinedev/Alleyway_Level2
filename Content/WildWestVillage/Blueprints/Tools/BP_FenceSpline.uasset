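; BP_FenceSpline is a construction-script tool that builds a straight fence sized to a spline's length.
; It derives section count from mesh bounds, places sections every fixed step along local X, and stretches the last to fill the remainder.
; Unseeded chance rolls choose valved, variant or default meshes, with naming from a pipe tool.
; Optional flags yaw the root toward spline point 1 or zero it, instead of following curves.
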(fn `UserConstructionScript`
  (bind (_returnvalue_min _returnvalue_max) (break `Box` (`StaticMesh.GetBoundingBox` (`self.Mesh_Input`))))
  (bind (_returnvalue_x _returnvalue_y) (`KismetMathLibrary.BreakVector` (`SplineComponent.GetLocationAtSplinePoint` (`self.InterSpline`) 1 "Local")))
  (bind _returnvalue (`SplineComponent.GetSplineLength` (`self.InterSpline`)))
  (bind _returnvalue_x_2 (`KismetMathLibrary.BreakVector` (+ (`KismetMathLibrary.Vector_GetAbs` _returnvalue_min) (`KismetMathLibrary.Vector_GetAbs` _returnvalue_max))))
  (set `self.Mesh_Input` null)
  (set `self.PipeMeshVar1` null)
  (set `self.PipeMeshVar2` null)
  (set `self.Calculator` 400.0)
  (bind _output_get (set `self.length` _returnvalue_x_2))
  (bind _returnvalue_2 (`KismetMathLibrary.FFloor` (/ (+ _returnvalue (/ (`self.Calculator`) 2.0)) (+ _output_get 0.0))))
  (bind _returnvalue_3 (* (- _returnvalue_2 1) (`self.Calculator`)))
  (bind _returnvalue_4 (`AddComponent|NODE_AddStaticMeshComponent-2` :`RelativeTransform` (`KismetMathLibrary.MakeTransform` (`KismetMathLibrary.MakeVector` (`KismetMathLibrary.Conv_IntToDouble` _returnvalue_3)) (struct) (`KismetMathLibrary.MakeVector` (/ (- _returnvalue _returnvalue_3) (`self.Calculator`)) 1.0 1.0))))
  (`StaticMeshComponent.SetStaticMesh` _returnvalue_4 (`self.Mesh_Input`))
  (for _index (range (+ (- _returnvalue_2 2) 1))
    (bind _returnvalue_5 (`AddComponent|NODE_AddStaticMeshComponent-0` :`RelativeTransform` (`KismetMathLibrary.MakeTransform` (`KismetMathLibrary.MakeVector` (`KismetMathLibrary.Conv_IntToDouble` (* _index (`self.Calculator`)))) (struct) (1.0 1.0 1.0))))
    (if (<= (`KismetMathLibrary.RandomInteger` 100) (`self.Valve Spawn Chance`))
      (`StaticMeshComponent.SetStaticMesh` _returnvalue_5 (`self.Valved Sections`))
      (else
        (if (<= (`KismetMathLibrary.RandomInteger` 100) (`self.Fence Variation 01 Spawn Chance`))
          (`StaticMeshComponent.SetStaticMesh` _returnvalue_5 (`self.PipeMeshVar1`))
          (elif (<= (`KismetMathLibrary.RandomInteger` 100) (`self.Fence Variation_02 Spawn Chance`))
            (`StaticMeshComponent.SetStaticMesh` _returnvalue_5 (`self.PipeMeshVar2`))
            (else
              (`StaticMeshComponent.SetStaticMesh` _returnvalue_5 (`self.Mesh_Input`)))))
        (if (`self.Set Angle`)
          (`SceneComponent.K2_SetWorldRotation` (`self.DefaultSceneRoot`) (`KismetMathLibrary.MakeRotator` 0.0 0.0 (`KismetMathLibrary.DegAtan` (/ _returnvalue_y _returnvalue_x))) false false)
          (elif (`self.Angle Reset 0`)
            (`SceneComponent.K2_SetWorldRotation` (`self.DefaultSceneRoot`) (`KismetMathLibrary.MakeRotator` 0.0) false false)))))))