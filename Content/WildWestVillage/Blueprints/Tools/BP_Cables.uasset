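; BP_Cables is a construction-time placement tool that spans a cable mesh between two spline points.
; When ActorSelected is set, the points snap to the base and target actors plus offsets.
; Spline length picks a small to extra-large mesh, taut or loose, with both styles sharing the extra-large one.
; The spawned mesh is aimed with a look-at rotation and stretched along X by length over bounding-box size.
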(fn `UserConstructionScript`
  (bind _spline (`self.Spline`))
  (bind (_returnvalue_min _returnvalue_max) (break `Box` (`StaticMesh.GetBoundingBox` (`self.Cable`))))
  (bind _returnvalue (`SplineComponent.GetLocationAtSplinePoint` _spline 0 "Local"))
  (bind _returnvalue_x (`KismetMathLibrary.BreakVector` (+ (`KismetMathLibrary.Vector_GetAbs` _returnvalue_min) (`KismetMathLibrary.Vector_GetAbs` _returnvalue_max))))
  (if (`self.Actor Selected`)
    (`SplineComponent.SetLocationAtSplinePoint` (`self.Spline`) 1 (+ (`self.K2_GetActorLocation` (`self.Actor Target`)) (`self.Target Offset`)) "World" true)
    (`SplineComponent.SetLocationAtSplinePoint` (`self.Spline`) 0 (+ (`self.K2_GetActorLocation` (`self.Actor Base`)) (`self.Base Offset`)) "World" true))
  (bind _output_get (set `self.Length` (`SplineComponent.GetDistanceAlongSplineAtSplinePoint` (`self.Spline`) 1)))
  (if (`self.LooseCable`)
    (bind _returnvalue_2 (<= _output_get 200.0))
    (if _returnvalue_2
      (set `self.Cable` "/Game/WildWestVillage/StaticMesh/Props/Cables/SM_Cable_S_loose.SM_Cable_S_loose")
      (else
        (bind _returnvalue_3 (< _output_get 375.0))
        (if _returnvalue_3
          (set `self.Cable` "/Game/WildWestVillage/StaticMesh/Props/Cables/SM_Cable_M_loose.SM_Cable_M_loose")
          (else
            (bind _returnvalue_4 (< _output_get 600.0))
            (if _returnvalue_4
              (set `self.Cable` "/Game/WildWestVillage/StaticMesh/Props/Cables/SM_Cable_L_loose.SM_Cable_L_loose")
              (else
                (bind _returnvalue_5 (>= _output_get 600.0))
                (if _returnvalue_5
                  _
                  (else
                    _))
                (set `self.Cable` "/Game/WildWestVillage/StaticMesh/Props/Cables/SM_Cable_xL.SM_Cable_xL" :!label _label)))))))
    (elif _returnvalue_2
      (set `self.Cable` "/Game/WildWestVillage/StaticMesh/Props/Cables/SM_Cable_S.SM_Cable_S")
      (elif _returnvalue_3
        (set `self.Cable` "/Game/WildWestVillage/StaticMesh/Props/Cables/SM_Cable_M.SM_Cable_M")
        (elif _returnvalue_4
          (set `self.Cable` "/Game/WildWestVillage/StaticMesh/Props/Cables/SM_Cable_L.SM_Cable_L")
          (elif _returnvalue_5
            (goto _label)
            (else
              (goto _label)))))))
  (bind _returnvalue_6 (`AddComponent|NODE_AddStaticMeshComponent-1` :`RelativeTransform` (`KismetMathLibrary.MakeTransform` _returnvalue (`KismetMathLibrary.FindLookAtRotation` _returnvalue (`SplineComponent.GetLocationAtSplinePoint` _spline 1 "Local")) (`KismetMathLibrary.MakeVector` (/ (`SplineComponent.GetDistanceAlongSplineAtSplinePoint` (`self.Spline`) 1) _returnvalue_x) 1.0 1.0))))
  (`StaticMeshComponent.SetStaticMesh` _returnvalue_6 (`self.Cable`)))