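; Rope prop that sizes a rope mesh to the distance of a referenced actor.
; The construction script moves spline point 1 to that actor's world location, then measures the spline length.
; That length, divided by a fixed base length, becomes the small rope mesh's Y scale.
; Mesh location and rotation stay as set, and there is no runtime logic.
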(fn `UserConstructionScript`
  (bind _returnvalue (`SceneComponent.GetRelativeTransform` (`self.SM_Rope_Small`)))
  (`SplineComponent.SetLocationAtSplinePoint` (`self.Spline`) 1 (`self.K2_GetActorLocation` (`self.Actor`)) "World" true)
  (bind _output_get (set `self.RopeLength` (`SplineComponent.GetSplineLength` (`self.Spline`))))
  (`SceneComponent.K2_SetRelativeTransform` (`self.SM_Rope_Small`) (`KismetMathLibrary.MakeTransform` (.location _returnvalue) (.rotation _returnvalue) (`KismetMathLibrary.MakeVector` (.x (.scale _returnvalue)) (* (/ _output_get 381.0) 1.0) (.z (.scale _returnvalue)))) false false))