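; Blockout spline tool that repeats a mesh along a spline as deformed spline mesh segments, with optional start and end cap meshes.
; The construction script splits the spline by Spacing, shortening tangents on the last partial segment, and takes scale from spline points and axis multipliers.
; Each segment's up vector comes from its midpoint, with end rolls relative to it, and a dynamic material receives a tiling parameter.
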(fn `UserConstructionScript`
  (locals (SegmentIndex :type Integer) (FinalTangentScale :type "Float (double-precision)") (SplineMeshComponent :type "SplineMeshComponent Object Reference") (StartDistance :type "Float (double-precision)") (MiddleDistance :type "Float (double-precision)") (EndDistance :type "Float (double-precision)"))
  (bind _spacing (`self.Spacing`))
  (bind _spacing_2 (`self.Spacing`))
  (bind _splinecomponent (`self.SplineComponent`))
  (bind _enddistance (`local.EndDistance`))
  (bind _startdistance (`local.StartDistance`))
  (bind _finaltangentscale (`local.FinalTangentScale`))
  (bind _splinemeshcomponent (`local.SplineMeshComponent`))
  (bind _splinecomponent_2 (`self.SplineComponent`))
  (bind _caprotate (`self.CapRotate`))
  (bind _capoffset (`self.CapOffset`))
  (bind _splinecomponent_3 (`self.SplineComponent`))
  (bind _splinecomponent_4 (`self.SplineComponent`))
  (bind _returnvalue (`SplineComponent.GetNumberOfSplinePoints` _splinecomponent_3))
  (bind (_remainder _returnvalue_2) (`KismetMathLibrary.FMod` (`SplineComponent.GetSplineLength` (`self.SplineComponent`)) _spacing))
  (bind _returnvalue_3 (`KismetMathLibrary.NegateRotator` (`SplineComponent.GetRotationAtDistanceAlongSpline` _splinecomponent_2 (`local.MiddleDistance`) "Local")))
  (for _index (range (+ _returnvalue_2 1))
    (set `self.TangentScale` _spacing)
    (bind _output_get (set `local.SegmentIndex` _index))
    ;[1 1 1] TangentScale
    (set `local.FinalTangentScale` (select `bool` (== _output_get _returnvalue_2) :`false` (`self.TangentScale`) :`true` (* (/ _remainder (`self.Spacing`)) (`self.TangentScale`))))
    ;[1 1 1] Segment Distance
    (bind _output_get_2 (set `local.StartDistance` (* (`local.SegmentIndex`) _spacing_2)))
    (set `local.MiddleDistance` (+ _output_get_2 (* _spacing_2 0.5)))
    (set `local.EndDistance` (+ (`local.StartDistance`) _spacing_2))
    ;[1 1 1] StaticMesh
    (bind _returnvalue_4 (`AddComponent|NODE_AddSplineMeshComponent-0`))
    (`SplineMeshComponent.SetForwardAxis` _returnvalue_4 (select `MovieScene3DPathSection_Axis` (`self.Axis`) :`X` "X" :`Y` "Y" :`Z` "Z" :`NEG_X` "X" :`NEG_Y` "Y" :`NEG_Z` "Z" :!type "ESplineMeshAxis Enum") true)
    (bind _output_get_3 (set `local.SplineMeshComponent` _returnvalue_4))
    (if (`self.CollisionEnable`)
      (`PrimitiveComponent.SetCollisionEnabled` _output_get_3 "QueryOnly"))
    (`StaticMeshComponent.SetStaticMesh` _output_get_3 (`self.Mesh`))
    (`SplineMeshComponent.SetStartAndEnd` (`local.SplineMeshComponent`) (`SplineComponent.GetLocationAtDistanceAlongSpline` _splinecomponent _startdistance "Local") (* (`SplineComponent.GetDirectionAtDistanceAlongSpline` _splinecomponent _startdistance "Local") _finaltangentscale) (`SplineComponent.GetLocationAtDistanceAlongSpline` _splinecomponent _enddistance "Local") (* (`SplineComponent.GetDirectionAtDistanceAlongSpline` _splinecomponent _enddistance "Local") _finaltangentscale) true)
    ;[1 1 1] Scale
    (`SplineMeshComponent.SetStartScale` _splinemeshcomponent (`KismetMathLibrary.MakeVector2D` (* (.y (`SplineComponent.GetScaleAtDistanceAlongSpline` (`self.SplineComponent`) (`local.StartDistance`))) (`self.Scale X`)) (* (.z (`SplineComponent.GetScaleAtDistanceAlongSpline` (`self.SplineComponent`) (`local.StartDistance`))) (`self.Scale Y`))) true)
    (`SplineMeshComponent.SetEndScale` _splinemeshcomponent (`KismetMathLibrary.MakeVector2D` (* (.y (`SplineComponent.GetScaleAtDistanceAlongSpline` (`self.SplineComponent`) (`local.EndDistance`))) (`self.Scale X`)) (* (.z (`SplineComponent.GetScaleAtDistanceAlongSpline` (`self.SplineComponent`) (`local.EndDistance`))) (`self.Scale Y`))) true)
    ;[1 1 1] MeshRoll
    (`SplineMeshComponent.SetSplineUpDir` _splinemeshcomponent (`SplineComponent.GetUpVectorAtDistanceAlongSpline` (`self.SplineComponent`) (`local.MiddleDistance`) "Local") true)
    (`SplineMeshComponent.SetStartRoll` _splinemeshcomponent (`KismetMathLibrary.DegreesToRadians` (.roll (`KismetMathLibrary.ComposeRotators` (`SplineComponent.GetRotationAtDistanceAlongSpline` _splinecomponent_2 (`local.StartDistance`) "Local") _returnvalue_3))) true)
    (`SplineMeshComponent.SetEndRoll` _splinemeshcomponent (`KismetMathLibrary.DegreesToRadians` (.roll (`KismetMathLibrary.ComposeRotators` (`SplineComponent.GetRotationAtDistanceAlongSpline` _splinecomponent_2 (`local.EndDistance`) "Local") _returnvalue_3))) true)
    ;[1 1 1] TileMaterial
    (bind _returnvalue_5 (`PrimitiveComponent.CreateDynamicMaterialInstance` (`local.SplineMeshComponent`) 0 null "None"))
    (`MaterialInstanceDynamic.SetScalarParameterValue` _returnvalue_5 (`KismetStringLibrary.Conv_StringToName` (`self.TileVarName`)) (`self.TileMaterial`)))
  ;[1 1 1] StartCap
  (if (`self.StartCap`)
    (bind _returnvalue_6 (`AddComponent|NODE_AddStaticMeshComponent-0`))
    (`StaticMeshComponent.SetStaticMesh` _returnvalue_6 (`self.StartCapMesh`))
    (`SceneComponent.K2_SetRelativeLocation` _returnvalue_6 (+ (`SplineComponent.GetLocationAndTangentAtSplinePoint` _splinecomponent_4 0 "Local") _capoffset) false false)
    (`SceneComponent.SetRelativeScale3D` _returnvalue_6 (`KismetMathLibrary.MakeVector` (* (.x (* (`SplineComponent.GetScaleAtSplinePoint` _splinecomponent_4 0) (`self.ScaleMinus`))) (`self.Scale X`)) (* (.y (* (`SplineComponent.GetScaleAtSplinePoint` _splinecomponent_4 0) (`self.ScaleMinus`))) (`self.Scale Y`)) (.z (* (`SplineComponent.GetScaleAtSplinePoint` _splinecomponent_4 0) (`self.ScaleMinus`)))))
    (`SceneComponent.K2_SetRelativeRotation` _returnvalue_6 (`KismetMathLibrary.ComposeRotators` (`KismetMathLibrary.Conv_VectorToRotator` _caprotate) (`SplineComponent.GetRotationAtSplinePoint` (`self.SplineComponent`) 0 "Local")) false false))
  ;[1 1 1] EndCap
  (if (`self.EndCap`)
    (bind _returnvalue_7 (`AddComponent|NODE_AddStaticMeshComponent-1`))
    (`StaticMeshComponent.SetStaticMesh` _returnvalue_7 (`self.EndCapMesh`))
    (`SceneComponent.K2_SetRelativeLocation` _returnvalue_7 (+ (`SplineComponent.GetLocationAndTangentAtSplinePoint` _splinecomponent_3 _returnvalue "Local") (* _capoffset -1.0)) false false)
    (`SceneComponent.SetRelativeScale3D` _returnvalue_7 (`KismetMathLibrary.MakeVector` (* (.x (`SplineComponent.GetScaleAtSplinePoint` _splinecomponent_3 _returnvalue)) (`self.Scale X`)) (* (.y (`SplineComponent.GetScaleAtSplinePoint` _splinecomponent_3 _returnvalue)) (`self.Scale Y`)) (.z (`SplineComponent.GetScaleAtSplinePoint` _splinecomponent_3 _returnvalue))))
    (`SceneComponent.K2_SetRelativeRotation` _returnvalue_7 (`KismetMathLibrary.ComposeRotators` (`KismetMathLibrary.Conv_VectorToRotator` (* _caprotate (-1.0 -1.0 -1.0))) (`SplineComponent.GetRotationAtSplinePoint` _splinecomponent_3 _returnvalue "Local")) false false)))