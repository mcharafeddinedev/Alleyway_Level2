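; BP_UnlockableDebris is a cart debris obstacle that the player clears with the IA_UnlockDebris input.
; Overlapping InteractToUnlockVolume calls EnableInput on the first-person character, not on the debris actor.
; If still locked, the input unlocks it, spawns sparks at fixed coordinates and plays the DebrisAnimation timeline.
; The timeline's first update jumps CartDebris far away and destroys the actor and blocking volume, so no gradual motion occurs.
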(event `self.InteractToUnlock Volume.OnComponentBeginOverlap`
  (params (OverlappedComponent :type "PrimitiveComponent Object Reference") (OtherActor :type "Actor Object Reference") (OtherComp :type "PrimitiveComponent Object Reference") (OtherBodyIndex :type Integer) (bFromSweep :type Boolean) (SweepResult :type "HitResult Structure (by ref)"))
  (bind _asbp_first_person_character (cast `/Game/FirstPerson/Blueprints/BP_FirstPersonCharacter` OtherActor))
  (`self.EnableInput` _asbp_first_person_character (`GameplayStatics.GetPlayerController` 0)))

(event `EnhancedInput|/Game/FirstPerson/Input/Actions/IA_UnlockDebris`
  (params (ActionValue :type Boolean) (ElapsedSeconds :type "Float (double-precision)") (TriggeredSeconds :type "Float (double-precision)") (InputAction :type "InputAction Object Reference" :default "/Game/FirstPerson/Input/Actions/IA_UnlockDebris.IA_UnlockDebris"))
  (:`Triggered`
    (if (`self.isLocked`)
      (set `self.isLocked` false)
      (`GameplayStatics.SpawnEmitterAtLocation` "/Game/StarterContent/Particles/P_Sparks.P_Sparks" (0.0 50.0 190.0) (struct :`Yaw` 10.0) (10.0 5.0 10.0))
      (`Timeline|DebrisAnimation`
        (:`Update`
          (`SceneComponent.K2_SetRelativeLocation` (`self.CartDebris`) (0.0 100000.0 0.0) false false)
          (`self.K2_DestroyActor`)
          (`ActorComponent.K2_DestroyComponent` (`self.Blocking Volume`)))))))

(fn `UserConstructionScript`)